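; BP_BaseAmmo is the base projectile for the space shooter, moving forward along its facing each Tick while CanMove is set.
; On overlap, obstacles always register a hit, while other actors pass through CanHit, which skips PowerUp, Ammo and IgnoreTag tags and destroys the other actor if tagged Bound.
; Hit spawns an explosion, plays pitch-randomized sound, hides and stops the projectile, which is destroyed after a short delay.
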(event `self.ReceiveActorBeginOverlap`
  (params (OtherActor :type "Actor Object Reference"))
  (if (`KismetArrayLibrary.Array_Contains` (`Actor.Tags` OtherActor) "Obstacle")
    (bind _particleeffect (`self.Hit` :!label _label))
    (`KismetSystemLibrary.Delay` 0.3)
    (`/Engine/EditorBlueprintResources/StandardMacros.IsValid` _particleeffect
      (:`Is Valid`
        (`ActorComponent.K2_DestroyComponent` _particleeffect))
      (:`Is Not Valid`
        _))
    (`self.K2_DestroyActor`)
    (else
      (`/Engine/EditorBlueprintResources/StandardMacros.IsValid` OtherActor
        (:`Is Valid`
          (bind _canhit (`self.CanHit` OtherActor))
          (if _canhit
            (goto _label)))))))

(event `self.ReceiveTick`
  (params (DeltaSeconds :type "Float (single-precision)"))
  (`self.Move` DeltaSeconds))

(fn `CanHit`
  (params (Collision :type "Actor Object Reference"))
  (returns (CanHit :type Boolean))
  (bind _tags (`Actor.Tags` Collision))
  (if (`KismetArrayLibrary.Array_Contains` (`Actor.Tags` Collision) "Bound")
    (`self.K2_DestroyActor` Collision)
    (elif (not (or (`KismetArrayLibrary.Array_Contains` _tags "PowerUp") (`KismetArrayLibrary.Array_Contains` _tags "Ammo")))
      (return (not (`KismetArrayLibrary.Array_Contains` (`Actor.Tags` Collision) (`self.IgnoreTag`)))))))

(fn `Hit`
  (returns (ParticleEffect :type "ParticleSystemComponent Object Reference"))
  (bind _hitsoundclip (`self.HitSoundClip`))
  (bind _returnvalue (`GameplayStatics.SpawnEmitterAtLocation` (`self.ExplosionEffect`) (`self.K2_GetActorLocation`)))
  (`/Engine/EditorBlueprintResources/StandardMacros.IsValid` _hitsoundclip
    (:`Is Valid`
      (`GameplayStatics.PlaySound2D` _hitsoundclip 0.5 (`KismetMathLibrary.RandomFloatInRange` 0.8 1.2) 0.0 null null))
    (:`Is Not Valid`
      _))
  (`SceneComponent.SetVisibility` (`self.Capsule`) false false)
  (`SceneComponent.SetVisibility` (`self.Mesh`) false false)
  (set `self.CanMove` false)
  (return _returnvalue))

(fn `Move`
  (params (A :type "Float (double-precision)"))
  (if (`self.CanMove`)
    (`self.K2_SetActorLocation` (+ (`self.K2_GetActorLocation`) (* (* A (`self.Speed`)) (`self.GetActorForwardVector`))))))

(fn `UserConstructionScript`)