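; Kamikaze enemy for the space shooter that homes in on the player, then commits to a straight run.
; BeginPlay caches player character 0 as BP_Player, and Tick calls Move every frame.
; While FollowPlayer is set and 2D distance exceeds MinDistanceFollow, it rotates toward the player and sets MoveDirection to its forward vector.
; Once inside that distance it clears FollowPlayer for good, keeping its last heading.
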(event `self.ReceiveBeginPlay`
  (bind _returnvalue (`GameplayStatics.GetPlayerCharacter` 0))
  (`parent.ReceiveBeginPlay`)
  (`/Engine/EditorBlueprintResources/StandardMacros.IsValid` _returnvalue
    (:`Is Valid`
      (bind _asbp_player (cast `/Game/SpaceShooter/Player/BP_Player` _returnvalue))
      (set `self.Player` _asbp_player))))

(event `self.ReceiveTick`
  (params (DeltaSeconds :type "Float (single-precision)"))
  (bind _returnvalue (`self.K2_GetActorLocation`))
  (bind _returnvalue_2 (`self.K2_GetActorLocation` (`self.Player`)))
  (`self.Move` DeltaSeconds)
  (`/Engine/EditorBlueprintResources/StandardMacros.IsValid` (`self.Player`)
    (:`Is Valid`
      (if (`self.FollowPlayer`)
        (if (< (`self.MinDistanceFollow`) (`KismetMathLibrary.Distance2D` (`KismetMathLibrary.Conv_VectorToVector2D` _returnvalue) (`KismetMathLibrary.Conv_VectorToVector2D` _returnvalue_2)))
          (`self.K2_SetActorRotation` (`KismetMathLibrary.FindLookAtRotation` _returnvalue _returnvalue_2))
          (set `self.MoveDirection` (`self.GetActorForwardVector`))
          (else
            (set `self.FollowPlayer` false)))))))

(fn `UserConstructionScript`
  (`parent.UserConstructionScript`))