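; Player projectile for the space shooter that turns a single spawn into a three-way spread shot.
; On BeginPlay it runs the parent logic, then spawns two BP_PlayerBaseAmmo actors at its own transform and rotates them locally by equal, opposite angles.
; The actor itself keeps its original heading as the center shot, with any other behavior left to the parent class.
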(event `self.ReceiveBeginPlay`
  (`parent.ReceiveBeginPlay`)
  (bind _returnvalue (`|SpawnActorFromClass` "/Game/SpaceShooter/Weapons/BP_PlayerBaseAmmo.BP_PlayerBaseAmmo_C" (`self.GetTransform`) "Undefined" "MultiplyWithRoot" null null))
  (`self.K2_AddActorLocalRotation` _returnvalue (struct :`Yaw` -10.0) false false)
  (bind _returnvalue_2 (`|SpawnActorFromClass` "/Game/SpaceShooter/Weapons/BP_PlayerBaseAmmo.BP_PlayerBaseAmmo_C" (`self.GetTransform`) "Undefined" "MultiplyWithRoot" null null))
  (`self.K2_AddActorLocalRotation` _returnvalue_2 (struct :`Yaw` 10.0) false false))

(fn `UserConstructionScript`
  (`parent.UserConstructionScript`))