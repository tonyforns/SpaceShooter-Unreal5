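; Enemy spawner for the space shooter that activates once the game controller's level reaches its base spawn level, playing a one-time alert sound.
; Tick runs a countdown, spawning the enemy class at a random point between Min and Max, oriented by SpawnDirection.
; OnLevelUp recomputes the delay with an inverted quadratic curve, shortening it from maximum toward minimum as levels rise.
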(event `self.ReceiveBeginPlay`
  (bind _returnvalue (`GameplayStatics.GetGameMode`))
  (set `self.DelayTimer` 0.0)
  (`/Engine/EditorBlueprintResources/StandardMacros.IsValid` _returnvalue
    (:`Is Valid`
      (bind _asss_game_controller (cast `/Game/SpaceShooter/SS_GameController` _returnvalue))
      (set `self.GameController` _asss_game_controller)
      (add `/Game/SpaceShooter/SS_GameController.OnLevelUp` _asss_game_controller (delegate `UpdateSpawnTime`)))))

(event `UpdateSpawnTime`
  (bind _returnvalue (`self.CanSpawn`))
  (if _returnvalue
    (`self.UpdateSpawnTimeFunction`)))

(event `self.ReceiveTick`
  (params (DeltaSeconds :type "Float (single-precision)"))
  (bind _returnvalue (`self.CanSpawn`))
  (if _returnvalue
    (set `self.DelayTimer` (- (`self.DelayTimer`) DeltaSeconds))
    (if (<= (`self.DelayTimer`) 0.0)
      (`self.SpawnActor`)
      (`self.SetDealy`))))

(fn `CanSpawn`
  (returns (ReturnValue :type Boolean))
  (bind _returnvalue (<= (`self.BaseLevelToSpawn`) (`/Game/SpaceShooter/SS_GameController.Level` (`self.GameController`))))
  (if (and _returnvalue (`self.IsFirstSpawn`))
    (set `self.IsFirstSpawn` false)
    (`GameplayStatics.PlaySound2D` "/Game/SpaceShooter/Audio/Alert.Alert" 2.0 (`KismetMathLibrary.RandomFloatInRange` 0.8 1.2) 0.0 null null))
  (return _returnvalue))

(fn `SetDealy`
  (set `self.DelayTimer` (`self.SpawnDelay`)))

(fn `SpawnActor`
  (bind _enemytospawn (`self.EnemyToSpawn`))
  (if (`KismetSystemLibrary.IsValidClass` _enemytospawn)
    (`|SpawnActorFromClass` _enemytospawn (`KismetMathLibrary.MakeTransform` (`KismetMathLibrary.VLerp` (`SceneComponent.K2_GetComponentLocation` (`self.Min`)) (`SceneComponent.K2_GetComponentLocation` (`self.Max`)) (`KismetMathLibrary.RandomFloatInRange` 0.0 1.0)) (`KismetMathLibrary.TransformRotation` (`SceneComponent.K2_GetComponentToWorld` (`self.SpawnDirection`)))) "Undefined" "MultiplyWithRoot" null null)))

(fn `UpdateSpawnTimeFunction`
  (bind _gamecontroller (`self.GameController`))
  (bind _minspawntime (`self.MinSpawnTime`))
  (set `self.SpawnDelay` (+ (* (- 1.0 (`KismetMathLibrary.MultiplyMultiply_FloatFloat` (/ (- (`KismetMathLibrary.Conv_IntToDouble` (- (`/Game/SpaceShooter/SS_GameController.Level` _gamecontroller) (`self.BaseLevelToSpawn`))) 1.0) (- (`/Game/SpaceShooter/SS_GameController.MAX_LEVEL` _gamecontroller) 1)) 2.0)) (- (`self.MaxSpawnTime`) _minspawntime)) _minspawntime)))

(fn `UserConstructionScript`)