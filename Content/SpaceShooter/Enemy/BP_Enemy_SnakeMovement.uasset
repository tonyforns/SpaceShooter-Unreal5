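; Space shooter enemy variant that weaves in a snake pattern and fires repeatedly, extending a parent enemy class.
; Each tick, it sets MoveDirection to its forward vector plus a sine-driven sideways offset, tuned by Frequency and Amplitud, then normalized.
; The Fire override triggers Refire, which after a short delay calls Fire again if an actor lookup is valid, forming a repeating chain that also decrements ShootTimer.
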(event `self.ReceiveBeginPlay`
  (`parent.ReceiveBeginPlay`)
  (set `self.MoveDirection` (`self.GetActorForwardVector`)))

(event `self.ReceiveActorBeginOverlap`
  (params (OtherActor :type "Actor Object Reference"))
  (`parent.ReceiveActorBeginOverlap` OtherActor))

(event `self.ReceiveTick`
  (params (DeltaSeconds :type "Float (single-precision)"))
  (`parent.ReceiveTick` DeltaSeconds)
  (bind _output_get (set `self.ElapseTime` (+ DeltaSeconds (`self.ElapseTime`))))
  (set `self.MoveDirection` (`KismetMathLibrary.Normal` (+ (`self.GetActorForwardVector`) (* (* (`KismetMathLibrary.DegSin` (* (`self.Frequency`) _output_get 360.0)) (`self.Amplitud`) 0.005) (`self.GetActorRightVector`))))))

(event `Refire`
  (`KismetSystemLibrary.Delay` 0.3)
  (`GameplayStatics.GetActorOfClass` null)
  (`/Engine/EditorBlueprintResources/StandardMacros.IsValid` null
    (:`Is Valid`
      (`self.Fire` null)
      (set `self.ShootTimer` (- (`self.ShootTimer`) 0.3)))))

(fn `Fire`
  (params (FirePoint :type "SceneComponent Object Reference"))
  (`parent.Fire` FirePoint)
  (`self.Refire`))

(fn `UserConstructionScript`
  (`parent.UserConstructionScript`))