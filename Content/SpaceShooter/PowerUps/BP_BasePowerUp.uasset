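; Base power-up actor for the space shooter, with an empty ApplyPowerUp function as the hook for specific effects.
; Each tick it moves along its forward vector at Speed, without sweeping.
; Overlapping a Player-tagged actor not tagged Ammo caches BP_Player, shows Message through SS_GameController and applies the effect.
; It then plays a sound, hides, disables collision and destroys itself after a short delay.
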(event `self.ReceiveActorBeginOverlap`
  (params (OtherActor :type "Actor Object Reference"))
  (bind _tags (`Actor.Tags` OtherActor))
  (if (`KismetArrayLibrary.Array_Contains` _tags "Ammo")
    _
    (elif (`KismetArrayLibrary.Array_Contains` _tags "Player")
      (`self.TryToGetPlayer` OtherActor)
      (`self.ShowPowerUpMessage`)
      (`self.ApplyPowerUp`)
      (`GameplayStatics.PlaySound2D` null 1.0 1.0 0.0 null null)
      (`SceneComponent.SetVisibility` (`self.DefaultSceneRoot`) false false)
      (`SceneComponent.SetVisibility` (`self.Mesh`) false false)
      (`PrimitiveComponent.SetCollisionEnabled` (`self.Collider`) "NoCollision")
      (`PrimitiveComponent.SetCollisionEnabled` (`self.Mesh`) "NoCollision")
      (`KismetSystemLibrary.Delay` 0.2)
      (`self.K2_DestroyActor`))))

(event `self.ReceiveTick`
  (params (DeltaSeconds :type "Float (single-precision)"))
  (`self.Move` DeltaSeconds))

(fn `ApplyPowerUp`)

(fn `Move`
  (params (A :type "Float (single-precision)"))
  (`self.K2_SetActorLocation` (+ (* A (`self.Speed`) (`self.GetActorForwardVector`)) (`self.K2_GetActorLocation`))))

(fn `ShowPowerUpMessage`
  (bind _returnvalue (`GameplayStatics.GetGameMode`))
  (`/Engine/EditorBlueprintResources/StandardMacros.IsValid` _returnvalue
    (:`Is Valid`
      (bind _asss_game_controller (cast `/Game/SpaceShooter/SS_GameController` _returnvalue))
      (`/Game/SpaceShooter/SS_GameController.ShowPowerUpMessage` _asss_game_controller (`self.Message`)))))

(fn `TryToGetPlayer`
  (params (Collision :type "Actor Object Reference"))
  (if (`KismetArrayLibrary.Array_Contains` (`Actor.Tags` Collision) "Player")
    (bind _asbp_player (cast `/Game/SpaceShooter/Player/BP_Player` (`GameplayStatics.GetPlayerCharacter` 0)))
    (set `self.Player` _asbp_player)))

(fn `UserConstructionScript`)