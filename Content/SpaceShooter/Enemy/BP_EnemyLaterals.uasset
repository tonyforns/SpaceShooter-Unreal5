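; BP_EnemyLaterals is a space shooter enemy that picks a random sideways direction and reverses it at the level bounds.
; BeginPlay sets MoveDirection to the Arrow's right vector or its negation, leaving the rest to the parent class.
; Overlapping an actor tagged Bound calls ChangeDirection, which flips the direction and compounds higher Speed and shorter ShootDelay on each bounce.
; Other overlaps pass to the parent.
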(event `self.ReceiveBeginPlay`
  (bind _returnvalue (`SceneComponent.GetRightVector` (`self.Arrow`)))
  (`parent.ReceiveBeginPlay`)
  (if (`KismetMathLibrary.RandomBool`)
    (set `self.MoveDirection` _returnvalue)
    (else
      (set `self.MoveDirection` (* _returnvalue (-1.0 -1.0 -1.0))))))

(event `self.ReceiveActorBeginOverlap`
  (params (OtherActor :type "Actor Object Reference"))
  (if (`KismetArrayLibrary.Array_Contains` (`Actor.Tags` OtherActor) "Bound")
    (`self.ChangeDirection`)
    (else
      (`parent.ReceiveActorBeginOverlap` OtherActor))))

(fn `ChangeDirection`
  (set `self.MoveDirection` (* (`self.MoveDirection`) (-1.0 -1.0 -1.0)))
  (set `self.ShootDelay` (* (`self.ShootDelay`) 0.8))
  (set `self.Speed` (* (`self.Speed`) 1.25)))

(fn `UserConstructionScript`
  (`parent.UserConstructionScript`))