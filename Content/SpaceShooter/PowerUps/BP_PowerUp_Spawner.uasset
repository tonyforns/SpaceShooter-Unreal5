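; Power-up spawner for the space shooter that spawns a random power-up whenever the game level reaches a multiple of four.
; It binds to the SS_GameController level-up event on BeginPlay.
; Each spawn picks a class from PowerUpToSpawn, places it at a random point between the Min and Max markers and takes its rotation from SpawnDirection.
; A countdown-based spawn function exists but is not wired up.
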(event `self.ReceiveBeginPlay`
  (bind _returnvalue (`GameplayStatics.GetGameMode`))
  (`/Engine/EditorBlueprintResources/StandardMacros.IsValid` _returnvalue
    (:`Is Valid`
      (bind _asss_game_controller (cast `/Game/SpaceShooter/SS_GameController` _returnvalue))
      (add `/Game/SpaceShooter/SS_GameController.OnLevelUp` _asss_game_controller (delegate `SpawnPowerUp`)))))

(event `SpawnPowerUp`
  (if (== (mod (`/Game/SpaceShooter/SS_GameController.Level` (stale `self.ReceiveBeginPlay` _asss_game_controller)) 4) 0)
    (`self.SpawnActor`)))

(event `self.ReceiveTick`
  (params (DeltaSeconds :type "Float (single-precision)")))

(fn `SpawnActor`
  (bind _outitem (`KismetArrayLibrary.Array_Random` (`self.PowerUpToSpawn`)))
  (if (`KismetSystemLibrary.IsValidClass` _outitem)
    (`|SpawnActorFromClass` _outitem (`KismetMathLibrary.MakeTransform` (`KismetMathLibrary.VLerp` (`SceneComponent.K2_GetComponentLocation` (`self.Min`)) (`SceneComponent.K2_GetComponentLocation` (`self.Max`)) (`KismetMathLibrary.RandomFloatInRange` 0.0 1.0)) (`KismetMathLibrary.TransformRotation` (`SceneComponent.K2_GetComponentToWorld` (`self.SpawnDirection`)))) "Undefined" "MultiplyWithRoot" null null)))

(fn `SpawnAfterTime`
  (params (B :type "Float (double-precision)"))
  (set `self.DelayTimer` (- (`self.DelayTimer`) B))
  (if (<= (`self.DelayTimer`) 0.0)
    (`self.SpawnActor`)
    (set `self.DelayTimer` (`self.SpawnDelay`))))

(fn `UserConstructionScript`)