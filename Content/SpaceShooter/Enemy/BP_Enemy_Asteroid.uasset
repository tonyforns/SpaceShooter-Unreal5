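; Asteroid enemy for the space shooter, a child Blueprint that varies its size, orientation and speed per instance.
; BeginPlay takes the move direction from the Arrow, then randomizes the BoxCollider's rotation and uniform scale and the Speed.
; Tick calls the parent and adds a fixed per-frame spin to the mesh, independent of delta time.
; Fire is empty, and the overlap event does nothing, leaving the parent's overlap call unreached.
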(event `self.ReceiveBeginPlay`
  (`parent.ReceiveBeginPlay`)
  (set `self.MoveDirection` (`SceneComponent.GetForwardVector` (`self.Arrow`)))
  (`SceneComponent.K2_SetWorldRotation` (`self.BoxCollider`) (`KismetMathLibrary.RandomRotator` false) false false)
  (`SceneComponent.SetWorldScale3D` (`self.BoxCollider`) (* (`KismetMathLibrary.Vector_One`) (`KismetMathLibrary.RandomFloatInRange` 1.0 2.0)))
  (set `self.Speed` (`KismetMathLibrary.RandomFloatInRange` 50.0 150.0)))

(event `self.ReceiveActorBeginOverlap`
  (params (OtherActor :type "Actor Object Reference")))

(event `self.ReceiveTick`
  (params (DeltaSeconds :type "Float (single-precision)"))
  (`parent.ReceiveTick` DeltaSeconds)
  (`SceneComponent.K2_AddWorldRotation` (`self.Mesh`) (struct :`Pitch` 0.1 :`Yaw` 0.1 :`Roll` 0.1) false false))

(fn `Fire`
  (params (FirePoint :type "SceneComponent Object Reference")))

(fn `UserConstructionScript`
  (`parent.UserConstructionScript`))