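; BP_PowerUp_BOOM is a space shooter power-up that sets off a "boom" effect when applied.
; It overrides ApplyPowerUp, calling the parent logic first, then spawning a BoomAmmo actor at its own location and playing a loud 2D explosion sound.
; The event graph holds only disabled stubs, so triggering is left to the parent class or external callers.
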(fn `ApplyPowerUp`
  (`parent.ApplyPowerUp`)
  (`|SpawnActorFromClass` (`self.BoomAmmo`) (`KismetMathLibrary.Conv_VectorToTransform` (`self.K2_GetActorLocation`)) "Undefined" "MultiplyWithRoot" null null)
  (`GameplayStatics.PlaySound2D` "/Game/StarterContent/Audio/Explosion02.Explosion02" 3.0 1.0 0.0 null null))

(fn `UserConstructionScript`
  (`parent.UserConstructionScript`))