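; Player ship for the space shooter, moved and fired through Enhanced Input, with a timer-gated cooldown between bullets.
; Tag-based overlaps cost a life on unshielded enemy hits, kill outright on obstacles and play a sound for power-ups.
; Separate events provide speed, fire-rate, heal and timed-shield boosts, with Tick counting down the shield.
; Damage and death fire notification calls, and death spawns an explosion before destroying the actor.
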(event `MovementSpeedUp`
  ; Power UP
  (set `self.Speed` (* (`self.Speed`) 1.2)))

(event `FireSpeedUp`
  ; Power UP
  (set `self.FIreDelay` (* (`self.FIreDelay`) 0.8)))

(event `ActiveShield`
  (bind _sm_shield (`self.SM_Shield`))
  ; SHIELD POWER UP
  (set `self.IsShieldUp` true)
  (`SceneComponent.SetVisibility` _sm_shield true false)
  (`PrimitiveComponent.SetCollisionEnabled` _sm_shield "QueryOnly")
  (set `self.ShieldTimer` 10.0)
  (`GameplayStatics.PlaySound2D` "/Game/SpaceShooter/Audio/ShieldUp_2.ShieldUp_2" 1.0 1.0 0.0 null null))

(event `DeactiveShield`
  (bind _sm_shield (`self.SM_Shield`))
  ; SHIELD POWER UP
  (set `self.IsShieldUp` false)
  (`SceneComponent.SetVisibility` _sm_shield false false)
  (`PrimitiveComponent.SetCollisionEnabled` _sm_shield "NoCollision")
  (`GameplayStatics.PlaySound2D` "/Game/SpaceShooter/Audio/ShieldDown.ShieldDown" 1.0 1.0 0.0 null null))

(event `self.ReceiveBeginPlay`
  ; OBJECT LIFE CICLE
  (bind _asplayer_controller (cast `PlayerController` (`self.GetController`)))
  (bind _returnvalue (pcsubsystem `EnhancedInputLocalPlayerSubsystem` _asplayer_controller))
  (`/Engine/EditorBlueprintResources/StandardMacros.IsValid` _returnvalue
    (:`Is Valid`
      (`EnhancedInputSubsystemInterface.AddMappingContext` _returnvalue "/Game/SpaceShooter/Inputs/IMC_Player.IMC_Player" 0 (struct))
      (bind _asss_game_controller (cast `/Game/SpaceShooter/SS_GameController` (`GameplayStatics.GetGameMode`)))
      (set `self.Game Controller` _asss_game_controller)
      (`self.DeactiveShield`))))

(event `self.ReceiveTick`
  (params (DeltaSeconds :type "Float (single-precision)"))
  ; OBJECT LIFE CICLE
  (`self.HandleShieldStatus` DeltaSeconds))

(event `self.ReceiveActorBeginOverlap`
  (params (OtherActor :type "Actor Object Reference"))
  (bind _tags (`Actor.Tags` OtherActor))
  ; OBJECT LIFE CICLE
  (if (`KismetArrayLibrary.Array_Contains` _tags "Enemy")
    (if (not (`self.IsShieldUp`))
      (`self.GetDamage`))
    (elif (`KismetArrayLibrary.Array_Contains` _tags "PowerUp")
      (`self.HundlePowerUp` OtherActor)
      (elif (`KismetArrayLibrary.Array_Contains` _tags "Obstacle")
        (set `self.Lifes` 1)
        (`self.GetDamage`)))))

(event `EnhancedInput|/Game/SpaceShooter/Inputs/IA_Player_Movement`
  (params (ActionValue :type "Vector2D Structure") (ElapsedSeconds :type "Float (double-precision)") (TriggeredSeconds :type "Float (double-precision)") (InputAction :type "InputAction Object Reference" :default "/Game/SpaceShooter/Inputs/IA_Player_Movement.IA_Player_Movement"))
  (bind _speed (`self.Speed`))
  ; IMPUT SYSTEM ACTIONS
  (:`Triggered`
    (`self.AddMovementInput` (* (`KismetMathLibrary.Vector_Right`) _speed) ActionValue_X)
    (`self.AddMovementInput` (* (`KismetMathLibrary.Vector_Forward`) _speed) ActionValue_Y)))

(event `EnhancedInput|/Game/SpaceShooter/Inputs/IA_Player_Fire`
  (params (ActionValue :type Boolean) (ElapsedSeconds :type "Float (double-precision)") (TriggeredSeconds :type "Float (double-precision)") (InputAction :type "InputAction Object Reference" :default "/Game/SpaceShooter/Inputs/IA_Player_Fire.IA_Player_Fire"))
  ; IMPUT SYSTEM ACTIONS
  (:`Triggered`
    (if (`self.CanFire`)
      (`self.DoFire`)
      (set `self.CanFire` false)
      (`KismetSystemLibrary.K2_SetTimerDelegate` (delegate `UpdateFire`) (`self.FIreDelay`)))))

(event `UpdateFire`
  ; IMPUT SYSTEM ACTIONS
  (set `self.CanFire` true))

(event `GetDamage`
  ; GET DEMAGE
  (bind _output_get (set `self.Lifes` (- (`self.Lifes`) 1)))
  (`self.OnPlayerDamaged`)
  (if (<= _output_get 0)
    (`self.OnPlayerDead`)
    (`self.PlayDead`)))

(event `Heal`
  (bind _lifes (`self.Lifes`))
  ; Heal
  (if (!= _lifes 3)
    (set `self.Lifes` (+ _lifes 1))
    (`self.OnPlayerDamaged`)))

(event `PlayDead`
  (`GameplayStatics.SpawnEmitterAtLocation` "/Game/StarterContent/Particles/P_Fire.P_Fire")
  (`GameplayStatics.PlaySound2D` "/Game/SpaceShooter/Audio/Explosion.Explosion" 1.0 1.0 0.0 null null)
  (`self.K2_DestroyActor`))

(fn `DoFire`
  (`|SpawnActorFromClass` (`self.Ammo`) (`SceneComponent.K2_GetComponentToWorld` (`self.BulletSpawn`)) "Undefined" "MultiplyWithRoot" null null)
  (`GameplayStatics.PlaySound2D` "/Game/SpaceShooter/Audio/Fire.Fire" 0.5 (`KismetMathLibrary.RandomFloatInRange` 0.8 1.2) 0.0 null null))

(fn `HandleShieldStatus`
  (params (B :type "Float (double-precision)"))
  (if (`self.IsShieldUp`)
    (set `self.ShieldTimer` (- (`self.ShieldTimer`) B))
    (if (<= (`self.ShieldTimer`) 0.0)
      (`self.DeactiveShield`))))

(fn `HundlePowerUp`
  (params (PowerUp :type "Actor Object Reference"))
  (`GameplayStatics.PlaySound2D` "/Game/SpaceShooter/Audio/BuyPowerUp.BuyPowerUp" 1.0 1.0 0.0 null null))

(fn `UserConstructionScript`)